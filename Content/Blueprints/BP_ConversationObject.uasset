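; BP_ConversationObject is a world actor that displays a configurable image on a plane and turns to face the player.
; The construction script creates a dynamic material instance on the plane and feeds Image into its texture parameter.
; Each tick, RotationTick smoothly interpolates the root toward the player pawn, using MakeRotFromZX to keep it upright.
; TargetState only stores the Targeted flag, which nothing in this graph reads.
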(event `self.ReceiveTick`
  (params (DeltaSeconds :type "Float (single-precision)"))
  (`self.RotationTick` DeltaSeconds))

(fn `RotationTick`
  (params (DeltaSeconds :type "Float (double-precision)"))
  (bind _defaultsceneroot (`self.DefaultSceneRoot`))
  (`SceneComponent.K2_SetWorldRotation` _defaultsceneroot (`KismetMathLibrary.RInterpTo` (`SceneComponent.K2_GetComponentRotation` _defaultsceneroot) (`KismetMathLibrary.MakeRotFromZX` (`KismetMathLibrary.Vector_Up`) (- (`self.K2_GetActorLocation` (`GameplayStatics.GetPlayerPawn` 0)) (`SceneComponent.K2_GetComponentLocation` _defaultsceneroot))) DeltaSeconds 5.0) false false))

(fn `TargetState`
  (params (State :type Boolean))
  (set `self.Targeted` State))

(fn `UserConstructionScript`
  (bind _plane (`self.Plane`))
  (bind _returnvalue (`PrimitiveComponent.CreateDynamicMaterialInstance` _plane 0 (`PrimitiveComponent.GetMaterial` _plane 0) "None"))
  (`MaterialInstanceDynamic.SetTextureParameterValue` _returnvalue "Image" (`self.Image`)))