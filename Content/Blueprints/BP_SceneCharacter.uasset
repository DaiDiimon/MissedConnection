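; BP_SceneCharacter is a player character that possesses itself on BeginPlay and moves relative to control yaw with mouse look.
; Holding Zoom enables controller-yaw rotation and interpolates the spring arm length to zero, restoring the original length on release.
; While zoomed, a camera line trace each tick finds BP_ConversationObject actors and sets their target state, clearing it when hitting other actors or releasing zoom.
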(event `self.ReceiveBeginPlay`
  (`Controller.Possess` (`GameplayStatics.GetPlayerController` 0) self)
  (set `self.OrigArmLength` (`SpringArmComponent.TargetArmLength` (`self.SpringArm`))))

(event `self.ReceiveTick`
  (params (DeltaSeconds :type "Float (single-precision)"))
  (`self.Zoom` DeltaSeconds)
  (`self.CO_Check`))

(event `InputAxis|Horizontal`
  (params (AxisValue :type "Float (single-precision)"))
  (`self.AddMovementInput` (`KismetMathLibrary.GetRightVector` (`KismetMathLibrary.MakeRotator` 0.0 0.0 (.yaw (`self.GetControlRotation`)))) AxisValue))

(event `InputAction|Interact`
  (params (Key :type "Key Structure")))

(event `InputAction|Zoom`
  (params (Key :type "Key Structure"))
  (bind _conversationobject (`self.ConversationObject`))
  (:`Pressed`
    (set `self.Zoomed` true)
    (set `self.bUseControllerRotationYaw` true))
  (:`Released`
    (set `self.Zoomed` false)
    (set `self.bUseControllerRotationYaw` false)
    (`/Engine/EditorBlueprintResources/StandardMacros.IsValid` _conversationobject
      (:`Is Valid`
        (`/Game/Blueprints/BP_ConversationObject.TargetState` _conversationobject false)
        (set `self.ConversationObject` null)))))

(event `InputAxis|MouseX`
  (params (AxisValue :type "Float (single-precision)"))
  (`self.AddControllerYawInput` AxisValue))

(event `InputAxis|MouseY`
  (params (AxisValue :type "Float (single-precision)"))
  (`self.AddControllerPitchInput` AxisValue))

(event `InputAxis|Vertical`
  (params (AxisValue :type "Float (single-precision)"))
  (`self.AddMovementInput` (`KismetMathLibrary.GetForwardVector` (`KismetMathLibrary.MakeRotator` 0.0 0.0 (.yaw (`self.GetControlRotation`)))) AxisValue))

(fn `CO_Check`
  (bind _camera (`self.Camera`))
  (bind _conversationobject (`self.ConversationObject`))
  (bind _returnvalue (`SceneComponent.K2_GetComponentLocation` _camera))
  (if (`self.Zoomed`)
    (bind (_outhit _returnvalue_2) (`KismetSystemLibrary.LineTraceSingle` _returnvalue (+ _returnvalue (* (`SceneComponent.GetForwardVector` _camera) 5000)) "TraceTypeQuery1"))
    (if _returnvalue_2
      (bind _asbp_conversation_object (cast `/Game/Blueprints/BP_ConversationObject` (`.HitActor` (`GameplayStatics.BreakHitResult` _outhit)))
        (:`then`
          (bind _output_get (set `self.ConversationObject` _asbp_conversation_object))
          (`/Game/Blueprints/BP_ConversationObject.TargetState` _output_get true))
        (:`CastFailed`
          (`/Engine/EditorBlueprintResources/StandardMacros.IsValid` _conversationobject
            (:`Is Valid`
              (`/Game/Blueprints/BP_ConversationObject.TargetState` _conversationobject false)
              (set `self.ConversationObject` null))))))))

(fn `UserConstructionScript`)

(fn `Zoom`
  (params (DeltaSeconds :type "Float (double-precision)"))
  (locals (TargetZoom :type "Float (double-precision)"))
  (bind _springarm (`self.SpringArm`))
  (bind _targetzoom (`local.TargetZoom`))
  (bind _targetarmlength (`SpringArmComponent.TargetArmLength` _springarm))
  (if (`self.Zoomed`)
    (set `local.TargetZoom` 0.0)
    (else
      (set `local.TargetZoom` (`self.OrigArmLength`))))
  (if (!= _targetzoom _targetarmlength)
    (set `SpringArmComponent.TargetArmLength` (`KismetMathLibrary.FInterpTo` _targetarmlength _targetzoom DeltaSeconds 30.0) _springarm)))