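; Conversation manager that stages a player-partner dialogue scene and presents its branching choices.
; StartConversation possesses the player, fades in audio, creates the conversation UI with a scene title, and hands that UI to both speakers.
; After a countdown, Tick passes the conversation asset's filename to ReadFile.
; The branch event switches to cursor-driven UI input and spawns one widget per choice, while the end event only prints a placeholder.
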(event `self.ReceiveBeginPlay`
  (`parent.ReceiveBeginPlay`))

(event `self.ReceiveTick`
  (params (DeltaSeconds :type "Float (single-precision)"))
  (bind _startcountdown (`self.Startcountdown`))
  (`parent.ReceiveTick` DeltaSeconds)
  (if (`self.Started`)
    _
    (elif (> _startcountdown 0.0)
      (set `self.Startcountdown` (- _startcountdown DeltaSeconds))
      (else
        (set `self.Started` true)
        (`self.ReadFile` (`DA_Conversation.filename` (`self.ConversationAsset`)))))))

(event `self.BranchBlueprint`
  (params (branches :type "Array of BranchInfo Structure (by ref)"))
  (bind _returnvalue (`GameplayStatics.GetPlayerController` 0))
  (bind _converesationui (`self.ConveresationUI`))
  (`WidgetBlueprintLibrary.SetInputMode_UIOnlyEx` _returnvalue null "LockOnCapture")
  (set `PlayerController.bShowMouseCursor` true _returnvalue)
  (`/Game/UI/ConversationUI.StartBranching` (`self.ConveresationUI`))
  (for _array_element branches
    (bind _returnvalue_2 (`|CreateWidget` "/Game/UI/BranchUI.BranchUI_C"))
    (`/Game/UI/BranchUI.Setup` _returnvalue_2 self _converesationui _array_element)
    (`/Game/UI/ConversationUI.AddBranch` _converesationui _returnvalue_2)))

(event `self.EndBlueprint`
  (`KismetSystemLibrary.PrintString` "END"))

(fn `SetupScene`
  (bind _conversationasset (`self.ConversationAsset`))
  (`AudioComponent.FadeIn` (`AmbientSound.AudioComponent` (`self.Audio`)) 3.0 1.0 0.0 "SCurve")
  (bind _returnvalue (`|CreateWidget` "/Game/UI/ConversationUI.ConversationUI_C"))
  (set `self.ConveresationUI` _returnvalue)
  (`/Game/UI/FaderUI.SetSceneText` (`/Game/UI/ConversationUI.FaderUI_31` _returnvalue) (`KismetStringLibrary.Concat_StrStr` (`KismetStringLibrary.Concat_StrStr` "Conversation " (`KismetMathLibrary.SelectString` "Inside: " "Outside: " (`DA_Conversation.inside` _conversationasset))) (`DA_Conversation.title` _conversationasset)))
  (`UserWidget.AddToViewport` _returnvalue 0))

(fn `SetupSpeakers`
  (bind _converesationui (`self.ConveresationUI`))
  (bind _asbp_conversation_player (cast `/Game/Blueprints/BP_ConversationPlayer` (`self.player`)))
  (bind _asbp_conversation_partner (cast `/Game/Blueprints/BP_ConversationPartner` (`self.partner`)))
  (set `/Game/Blueprints/BP_ConversationSpeaker.ConversationUI` _converesationui (`/Game/Blueprints/BP_ConversationPlayer.BP_ConversationSpeaker` _asbp_conversation_player))
  (set `/Game/Blueprints/BP_ConversationSpeaker.ConversationUI` _converesationui (`/Game/Blueprints/BP_ConversationPartner.BP_ConversationSpeaker` _asbp_conversation_partner)))

(fn `Start Conversation`
  (`Controller.Possess` (`GameplayStatics.GetPlayerController` 0) (`self.player`))
  (`self.SetupScene`)
  (`self.SetupSpeakers`))