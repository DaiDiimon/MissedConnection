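; Scene manager for Missed Connection that sets up an explorable scene and handles the transition into conversation levels.
; SetupScene possesses the Player, fades in audio and creates the scene UI, linking it to the LoadVolume.
; LoadConversation stores the conversation, viewed title and return level on the GameInstance, then fades out audio and UI.
; After a delay, it opens the inside, outside or final-solo level chosen by the conversation's flags.
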(event `self.ReceiveBeginPlay`
  (set `/Game/Blueprints/BP_SceneCharacter.SceneManager` self (`self.Player`)))

(event `LoadConversation`
  (params (Conversation :type "DA_Conversation Object Reference"))
  (bind _sceneui (`self.SceneUI`))
  (bind _asmissed_connection_game_instance (cast `MissedConnectionGameInstance` (`GameplayStatics.GetGameInstance`)))
  (`BlueprintSetLibrary.Set_Add` (`MissedConnectionGameInstance.viewed_conversations` _asmissed_connection_game_instance) (`DA_Conversation.title` Conversation))
  (set `MissedConnectionGameInstance.conversation_to_load` Conversation _asmissed_connection_game_instance)
  (bind _returnvalue (`GameplayStatics.GetCurrentLevelName` true))
  (set `MissedConnectionGameInstance.scene_to_return_to` _returnvalue _asmissed_connection_game_instance)
  (`AudioComponent.FadeOut` (`AmbientSound.AudioComponent` (`self.Audio`)) 3.0 0.0 "SCurve")
  (`/Game/UI/FaderUI.FadeOut` (`/Game/UI/SceneUI.FaderUI` _sceneui))
  (`/Game/UI/SceneUI.Remember` _sceneui false)
  (`KismetSystemLibrary.Delay` 3.0)
  (bind _levelname (`self.ConversationToLevelName` Conversation))
  (`GameplayStatics.OpenLevel` (`KismetStringLibrary.Conv_StringToName` _levelname)))

(fn `ConversationToLevelName`
  (params (Conversation :type "DA_Conversation Object Reference"))
  (returns (LevelName :type String))
  (if (`DA_Conversation.inside` Conversation)
    (return "ConversationInside")
    (elif (`DA_Conversation.final_A_solo` Conversation)
      (return "ConversationFinalA")
      (elif (`DA_Conversation.final_B_solo` Conversation)
        (return "ConversationFinalB")
        (else
          (return "ConversationOutside"))))))

(fn `Setup Scene`
  (`Controller.Possess` (`GameplayStatics.GetPlayerController` 0) (`self.Player`))
  (`AudioComponent.FadeIn` (`AmbientSound.AudioComponent` (`self.Audio`)) 3.0 1.0 0.0 "SCurve")
  (bind _returnvalue (`|CreateWidget` "/Game/UI/SceneUI.SceneUI_C"))
  (bind _output_get (set `self.SceneUI` _returnvalue))
  (set `/Game/Blueprints/BP_LoadVolume.SceneUI` _output_get (`self.LoadVolume`))
  (set `/Game/UI/SceneUI.SceneManager` self _output_get)
  (`/Game/UI/FaderUI.SetSceneText` (`/Game/UI/SceneUI.FaderUI` _output_get) (`self.SceneName`))
  (`UserWidget.AddToViewport` _returnvalue 0))