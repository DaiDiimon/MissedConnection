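; Conversation partner Blueprint: a character that can be animated, made to look and given a voice during conversations.
; PlayAnimation and Look cast the skeletal mesh's anim instance to AnimBP_HumanConvo and set its animation state, looking state and look blend.
; The construction script passes the AudioComponent to the BPConversationSpeaker.
; It has no active BeginPlay or Tick logic, so its events rely on external callers.
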(event `self.ReceiveBeginPlay`)

(event `self.PlayAnimation`
  (params (animation :type "EConversationAnimation Enum" :default "IDLE"))
  (bind _asanim_bp_human_convo (cast `/Game/Animations/AnimBP_HumanConvo` (`SkeletalMeshComponent.GetAnimInstance` (`self.SkeletalMesh`))))
  (set `/Game/Animations/AnimBP_HumanConvo.AnimationState` animation _asanim_bp_human_convo))

(event `self.Look`
  (params (state :type Boolean) (time :type "Float (single-precision)"))
  (bind _asanim_bp_human_convo (cast `/Game/Animations/AnimBP_HumanConvo` (`SkeletalMeshComponent.GetAnimInstance` (`self.SkeletalMesh`))))
  (set `/Game/Animations/AnimBP_HumanConvo.Looking` state _asanim_bp_human_convo)
  (set `/Game/Animations/AnimBP_HumanConvo.LookBlend` time _asanim_bp_human_convo))

(fn `UserConstructionScript`
  (bind _output_get (set `self.speaker` (`self.BP_ConversationSpeaker`)))
  (`ConversationSpeaker.SetAudioComponent` _output_get (`self.audio_component`)))