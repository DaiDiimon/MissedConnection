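; BP_ConversationSpeaker represents one speaker in a conversation and relays its dialogue events to a conversation UI.
; Start, update and end events call the matching ConversationUI functions, passing the LeftSpeaker value to indicate the speaker's side, plus the text on updates.
; BeginPlay and Tick only call their parent implementations.
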(event `self.ReceiveBeginPlay`
  (`parent.ReceiveBeginPlay`))

(event `self.ReceiveTick`
  (params (DeltaSeconds :type "Float (single-precision)"))
  (`parent.ReceiveTick` DeltaSeconds))

(event `self.EndDialogueUI`
  (`/Game/UI/ConversationUI.PlayDialogueEnd` (`self.ConversationUI`) (`self.left_speaker`)))

(event `self.StartDialogueUI`
  (`/Game/UI/ConversationUI.PlayDialogueStart` (`self.ConversationUI`) (`self.left_speaker`)))

(event `self.UpdateDialogueUI`
  (params (text :type String))
  (`/Game/UI/ConversationUI.UpdateText` (`self.ConversationUI`) (`self.left_speaker`) text))